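; Goblin NPC pawn that feeds what it senses to its BP_AICon AI controller, and only acts while alive.
; Pawn sensing passes seen pawns to the controller as the target actor.
; Noises above a volume threshold go through a SetDestination event, which updates the controller's target location.
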(event `self.MyPawnSensing.OnHearNoise`
  (params (Instigator :type "Pawn Object Reference") (Location :type "Vector Structure (by ref)") (Volume :type "Float (single-precision)"))
  (if (and (> Volume 300.0) (`self.IsAlive`))
    (`self.SetDestination` Location)))

(event `self.MyPawnSensing.OnSeePawn`
  (params (Pawn :type "Pawn Object Reference"))
  (if (`self.IsAlive`)
    (bind _asbp_aicon (cast `/Game/Blueprints/AI/BehaviorTree/BP_AICon` (`AIBlueprintHelperLibrary.GetAIController` self)))
    (`/Game/Blueprints/AI/BehaviorTree/BP_AICon.UpdateTargetActor` _asbp_aicon Pawn)))

(event `self.SetDestination`
  (params (Destination :type "Vector Structure"))
  (if (`self.IsAlive`)
    (bind _asbp_aicon (cast `/Game/Blueprints/AI/BehaviorTree/BP_AICon` (`AIBlueprintHelperLibrary.GetAIController` self)))
    (`/Game/Blueprints/AI/BehaviorTree/BP_AICon.UpdateTargetLocation` _asbp_aicon Destination)))

(fn `UserConstructionScript`
  (`parent.UserConstructionScript`))