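; Goblin enemy NPC that wanders random nearby navmesh points and chases sensed pawns to attack with a spike club montage.
; A delay-throttled Tick drives AI MoveTo, attacking on arrival and dropping the target when line of sight is lost.
; Pawn sensing sets targets on sight and redirects wandering toward loud noises.
; Player hits turn it toward the damage causer and play a hit or falldown montage, based on the player's melee index.
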(event `self.OnDamaged`
  (params (DamageAmount :type "Float (single-precision)") (HitInfo :type "HitResult Structure (by ref)") (InstigaterCharacter :type "TP_ThirdPersonCharacter Object Reference") (DamageCauser :type "Actor Object Reference"))
  (bind (_returnvalue_roll _returnvalue_pitch _returnvalue_yaw) (`KismetMathLibrary.BreakRotator` (`KismetMathLibrary.FindLookAtRotation` (`self.K2_GetActorLocation`) (`self.K2_GetActorLocation` DamageCauser))))
  (`parent.OnDamaged` DamageAmount HitInfo InstigaterCharacter DamageCauser)
  (bind _asbp_player_character (cast `/Game/Blueprints/BP_PlayerCharacter` InstigaterCharacter))
  (`self.PlayAnimMontage` (select `bool` (== (`/Game/Blueprints/BP_PlayerCharacter.MeleeIndex_0` _asbp_player_character) 3) :`false` "/Game/Animations/NPC/AM_Guardian_Hit.AM_Guardian_Hit" :`true` "/Game/Animations/NPC/AM_Guardian_Falldown.AM_Guardian_Falldown" :!type "AnimMontage Object Reference") 1.0 (`KismetStringLibrary.Conv_StringToName` (`KismetStringLibrary.Conv_IntToString` (`KismetMathLibrary.RandomIntegerInRange` 0 1))))
  (`self.K2_SetActorRotation` (`KismetMathLibrary.MakeRotator` 0.0 0.0 _returnvalue_yaw)))

(event `MeleeAttack`
  (bind _returnvalue (`SkeletalMeshComponent.GetAnimInstance` (`self.Mesh`)))
  (if (`self.IsMelee`)
    (if (not (`AnimInstance.IsAnyMontagePlaying` _returnvalue))
      (set `self.MeleeIndex` 0)
      (set `self.IsMelee` false)
      (`self.MeleeAttack`))
    (elif (not (> (`self.MeleeIndex`) 0))
      (`AnimInstance.Montage_Play` _returnvalue "/Game/Enemy/Enemy_Gruntling_Guardian/Animation/AM_SpikeClub_Attack.AM_SpikeClub_Attack" 1.0 "MontageLength" 0.0 true)
      (set `self.MeleeIndex` 1)
      (set `self.IsMelee` true))))

(event `self.ReceiveTick`
  (params (DeltaSeconds :type "Float (single-precision)"))
  (bind _targetpawn (`self.TargetPawn`))
  (bind _targetpawn_2 (`self.TargetPawn`))
  (`parent.ReceiveTick` DeltaSeconds)
  (`KismetSystemLibrary.Delay` 0.2)
  (if (`self.IsAlive`)
    (`|ExecutionSequence`
      (:`then_0`
        (`/Engine/EditorBlueprintResources/StandardMacros.IsValid` _targetpawn
          (:`Is Valid`
            (`|AIMoveTo` self (0.0 0.0 0.0) _targetpawn 30.0 true
              (:`OnSuccess`
                (`self.MeleeAttack`))))
          (:`Is Not Valid`
            (bind _movementresult (`|AIMoveTo` self (`self.Destination`) null 30.0 true)
              (:`then`
                (switch `EPathFollowingResult` _movementresult
                  (:`Success`
                    _)
                  (:`Aborted`
                    (`KismetSystemLibrary.Delay` 0.2)
                    (switch `EPathFollowingResult` _movementresult
                      (:`Aborted`
                        _))))
                (`self.GetNextNavPoint`))))))
      (:`then_1`
        (`/Engine/EditorBlueprintResources/StandardMacros.IsValid` _targetpawn_2
          (:`Is Valid`
            (bind _returnvalue (`MyPawnSensingComponent.HasLineOfSightTo_BP` (`self.MyPawnSensing`) _targetpawn_2))
            (if (not _returnvalue)
              (set `self.TargetPawn` null))))))))

(event `self.MyPawnSensing.OnSeePawn`
  (params (Pawn :type "Pawn Object Reference"))
  (set `self.TargetPawn` Pawn))

(event `self.MyPawnSensing.OnHearNoise`
  (params (Instigator :type "Pawn Object Reference") (Location :type "Vector Structure (by ref)") (Volume :type "Float (single-precision)"))
  (if (> Volume 300.0)
    (`self.SetDestination` Location)))

(fn `AttachWeapon`
  (params (SocketName :type Name) (Index :type Integer))
  (`parent.AttachWeapon` (`self.Name`) Index))

(fn `GetNextNavPoint`
  (bind (_randomlocation _returnvalue) (`NavigationSystemV1.K2_GetRandomReachablePointInRadius` (`self.K2_GetActorLocation`) 300.0 null null))
  (if _returnvalue
    (`self.SetDestination` _randomlocation)
    (else
      (`self.GetNextNavPoint`))))

(fn `SetDestination`
  (params (Destination :type "Vector Structure"))
  (bind _output_get (set `self.Destination` Destination))
  (`KismetSystemLibrary.DrawDebugSphere` _output_get 10.0 12 (struct :`R` 1.0 :`G` 0.817408 :`A` 1.0) 10.0 2.0))

(fn `UserConstructionScript`
  (`parent.UserConstructionScript`))