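; Melee weapon actor that damages actors its capsule overlaps during an attack, skipping actors of the wielder's own class.
; Begin and end attack events toggle the attacking flag and capsule collision, and also store hit-delay settings unused here.
; A DoOnce limits damage to one hit until 0.2 seconds after an overlap ends.
; Each hit credits the third-person character's controller and calls HitPause, which is empty here.
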(event `self.ReceiveActorBeginOverlap`
  (params (OtherActor :type "Actor Object Reference"))
  (if (and (!= (`GameplayStatics.GetObjectClass` OtherActor) (`GameplayStatics.GetObjectClass` (`self.GetInstigator`))) (`self.IsAttacking`))
    (`/Engine/EditorBlueprintResources/StandardMacros.DoOnce` false :!label _label
      (:`Completed`
        (`GameplayStatics.ApplyDamage` OtherActor (`self.Damage`) (`Pawn.GetController` (cast `TP_ThirdPersonCharacter` (`self.GetInstigator`) :!pure true)) self)
        (`self.HitPause`)))))

(event `HitPause`)

(event `self.ReceiveActorEndOverlap`
  (params (OtherActor :type "Actor Object Reference"))
  (`KismetSystemLibrary.Delay` 0.2)
  (goto _label :!via `Reset`))

(event `BeginWeaponAttack`
  (params (AttackDelayCount :type Integer) (AttackDelayTime :type "Float (double-precision)"))
  (set `self.AttackDelayCount` AttackDelayCount)
  (set `self.AttackDelayTime` AttackDelayTime)
  (set `self.IsAttacking` true)
  (`PrimitiveComponent.SetCollisionEnabled` (`self.CapsuleCollision`) "QueryOnly"))

(event `EndWeaponAttack`
  (set `self.IsAttacking` false)
  (`PrimitiveComponent.SetCollisionEnabled` (`self.CapsuleCollision`) "NoCollision"))

(fn `UserConstructionScript`)