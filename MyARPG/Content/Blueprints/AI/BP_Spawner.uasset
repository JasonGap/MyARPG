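; Wave spawner actor that releases groups of goblins over a set number of rounds.
; Delay-throttled Tick prunes dead goblins and, once all are dead, waits briefly, decrements Rounds and spawns the next wave.
; When rounds run out, it replaces its Tags with DeadTags.
; GoblinFactory picks random reachable points within SpawnRadius and line-traces down against static geometry to place each goblin on the ground.
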(event `self.ReceiveTick`
  (params (DeltaSeconds :type "Float (single-precision)"))
  (bind _spawnedgoblin (`self.SpawnedGoblin`))
  (`KismetSystemLibrary.Delay` 0.2)
  (if (`self.IsAllDead`)
    (`KismetSystemLibrary.Delay` (`KismetMathLibrary.RandomFloatInRange` 1.0 2.0))
    (bind _result (`/Engine/EditorBlueprintResources/StandardMacros.DecrementInt` (`self.Rounds`))
      (:`  `
        (if (> _result 0)
          (`self.GoblinFactory`)
          (set `self.IsAllDead` false)
          (else
            (set `self.Tags` (`self.DeadTags`))))))
    (elif (> (`KismetArrayLibrary.Array_Length` _spawnedgoblin) 0)
      (for _array_element _spawnedgoblin
        (if (not (`/Game/Blueprints/BP_Character.IsAlive` _array_element))
          (`KismetArrayLibrary.Array_RemoveItem` _spawnedgoblin _array_element)))
      (else
        (set `self.IsAllDead` true)))))

(fn `GoblinFactory`
  (bind _num (`self.Num`))
  (bind (_randomlocation _returnvalue) (`NavigationSystemV1.K2_GetRandomReachablePointInRadius` (.location (`self.GetTransform`)) (`self.SpawnRadius`) null null))
  (if (> _num 0)
    (for _ (range _num)
      (if _returnvalue
        (bind _output_get (set `self.SpawnLocation` _randomlocation))
        (bind (_outhit _returnvalue_2) (`KismetSystemLibrary.LineTraceSingleForObjects` (+ _output_get (0.0 0.0 900.0)) (`KismetMathLibrary.MakeVector` (.x (`self.SpawnLocation`)) (.y (`self.SpawnLocation`))) (`|MakeArray` "ObjectTypeQuery1" :!type "EObjectTypeQuery Enum")))
        (if _returnvalue_2
          (bind _returnvalue_3 (`|SpawnActorFromClass` (`self.Goblin`) (`KismetMathLibrary.MakeTransform` (`.Location` (`GameplayStatics.BreakHitResult` _outhit)) (.rotation (`self.GetTransform`)) (.scale (`self.GetTransform`))) "AlwaysSpawn" "OverrideRootScale" self null))
          (`KismetArrayLibrary.Array_Add` (`self.SpawnedGoblin`) _returnvalue_3))))))

(fn `UserConstructionScript`)