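; Player character Blueprint that handles a hammer melee combo on the NormalAttack input, plus an HP-based IsAlive check.
; DoMeleeAttack starts the attack montage, or calls JumpSectionforCombo when already in melee.
; With a valid JumpSectionNotify and the combo period enabled, that function queues a random next montage section from the notify's list.
; It also parses MeleeIndex from the section name's last character and prints it.
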(event `InputAction|NormalAttack`
  (params (Key :type "Key Structure"))
  (:`Pressed`
    (`self.DoMeleeAttack`)))

(fn `DoMeleeAttack`
  (bind _returnvalue (`SkeletalMeshComponent.GetAnimInstance` (`self.Mesh`)))
  (if (`self.IsMelee`)
    (`self.JumpSectionforCombo`)
    (if (not (`AnimInstance.IsAnyMontagePlaying` _returnvalue))
      (`AnimInstance.Montage_Play` _returnvalue "/Game/Characters/Animations/AM_Attack_Hammer.AM_Attack_Hammer" 1.0 "Duration" 0.0 true :!label _label)
      (set `self.MeleeIndex` 1)
      (set `self.IsMelee` true))
    (elif (not (> (`self.MeleeIndex`) 0))
      (goto _label))))

(fn `IsAlive`
  (returns (NewParam :type Boolean))
  (if (<= (`self.HP`) 0.0)
    (return false)
    (else
      (return true))))

(fn `JumpSectionforCombo`
  (bind _jumpsectionnotify (`self.JumpSectionNotify`))
  (bind _returnvalue (`SkeletalMeshComponent.GetAnimInstance` (`self.Mesh`)))
  (bind _jumpsections (`/Game/Blueprints/AnimMotifies/JumpSectionNS.JumpSections` _jumpsectionnotify))
  (bind _returnvalue_2 (`AnimInstance.GetCurrentActiveMontage` _returnvalue))
  (`/Engine/EditorBlueprintResources/StandardMacros.IsValid` _jumpsectionnotify
    (:`Is Valid`
      (if (`self.EnableComboPeriod`)
        (bind _output_get (set `self.NextSectionName` (`|GetArrayItem` _jumpsections (`KismetMathLibrary.RandomInteger` (`KismetArrayLibrary.Array_Length` _jumpsections)))))
        (bind _returnvalue_3 (`KismetStringLibrary.Conv_NameToString` _output_get))
        (bind _output_get_2 (set `self.MeleeIndex` (`KismetStringLibrary.Conv_StringToInt` (`KismetStringLibrary.GetSubstring` _returnvalue_3 (- (`KismetStringLibrary.Len` _returnvalue_3) 1)))))
        (`KismetSystemLibrary.PrintString` (`KismetStringLibrary.Conv_IntToString` _output_get_2))
        (`AnimInstance.Montage_SetNextSection` _returnvalue (`AnimInstance.Montage_GetCurrentSection` _returnvalue _returnvalue_2) (`self.NextSectionName`) _returnvalue_2)))))

(fn `UserConstructionScript`
  (`parent.UserConstructionScript`))